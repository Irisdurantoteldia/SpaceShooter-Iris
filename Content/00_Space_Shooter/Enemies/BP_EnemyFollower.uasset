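; Follower enemy for the space shooter, extending a parent Blueprint whose BeginPlay it calls first.
; On BeginPlay, Scanner rotates the Sphere component once to face the player character's mesh.
; MovementVector is then set from the normalized player-to-sphere direction multiplied by a zero vector, so it always ends up zero.
; Tick and overlap events are disabled stubs, so this graph never updates the aim afterward.
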(event EventBeginPlay
  (|CallParentFunction)
  (CallFunction|Scanner)
  (Variables|Default|SetMovementVector (* (Math|Vector|Normalize (- (Transformation|GetWorldLocation (Variables|Default|GetSphere)) (Transformation|GetWorldLocation (Variables|/Script/Engine.Character|GetMesh (Game|GetPlayerCharacter 0))))) "")))

(event Collision|EventActorBeginOverlap
  (params (OtherActor :type Actor%20Object%20Reference))
  (|CallParentFunction OtherActor) ; Este nodo está deshabilitado y no se le llamará.\nArrastra pines para construir una funcionalidad.
)

(event EventTick
  (params (DeltaSeconds :type Float%20%28single-precision%29))
  (|CallParentFunction DeltaSeconds) ; Este nodo está deshabilitado y no se le llamará.\nArrastra pines para construir una funcionalidad.
)

(fn ConstructionScript
  (|CallParentFunction))

(fn Scanner
  (Transformation|SetWorldRotation (Variables|Default|GetSphere) (Math|Rotator|FindLookatRotation (Transformation|GetWorldLocation (Variables|Default|GetSphere)) (Transformation|GetWorldLocation (Variables|/Script/Engine.Character|GetMesh (Game|GetPlayerCharacter 0)))) false false))